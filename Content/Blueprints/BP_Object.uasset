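; BP_Object is an actor with a Niagara component that receives velocity bounds from the AR trail subsystem.
; On BeginPlay it binds to the subsystem's trail-parsing-finished delegate, then copies the maximum and minimum trail velocities into the MaxSpeed and MinSpeed parameters.
; An unconnected projectile path prediction would fill the Niagara positions array but never runs, and the Running function is an empty stub.
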(event `self.ReceiveBeginPlay`
  ; Bind Json Parsing Delegate to the custom event
  (add `ARTrailSubsystem.OnTrailsParsedFinished` (subsystem `ARTrailSubsystem`) (delegate `CustomEvent`)))

(event `CustomEvent`
  (params (bSuccess :type Boolean) (Message :type String) (PointsNum :type Integer))
  (bind _returnvalue (subsystem `ARTrailSubsystem`))
  ; Bind Json Parsing Delegate to the custom event
  (`FXSystemComponent.SetFloatParameter` (`self.Niagara`) "MaxSpeed" (`ARTrailSubsystem.GetMaxTrailVelocity` _returnvalue))
  (`FXSystemComponent.SetFloatParameter` (`self.Niagara`) "MinSpeed" (`ARTrailSubsystem.GetMinTrailVelocity` _returnvalue)))

(fn `Running`
  (params (bInAdvanced :type Boolean))
  (returns (Output :type Boolean)))

(fn `UserConstructionScript`)