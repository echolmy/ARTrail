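; BP_Pawn is a mouse-driven camera pawn that supports rotating, drag-panning and zooming.
; Right-drag rotates the view, sending yaw to the Arrow and pitch to the SpringArm, and takes priority over left-drag.
; Left-drag moves the actor against mouse movement along the Arrow's right and forward vectors, scaled by MoveSpeed.
; The wheel changes spring arm length by SpeedWheel, with no clamping on zoom or pitch in the graph.
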(event `InputAxisKey|MouseX`
  (params (AxisValue :type "Float (single-precision)"))
  (bind _arrow (`self.Arrow`))
  (bind (_returnvalue_roll _returnvalue_pitch _returnvalue_yaw) (`KismetMathLibrary.BreakRotator` (`SceneComponent.K2_GetComponentRotation` _arrow)))
  ;[1 1 1] Rotation
  (if (`self.RightClick`)
    (`SceneComponent.K2_SetWorldRotation` _arrow (`KismetMathLibrary.MakeRotator` 0.0 _returnvalue_pitch (+ (* AxisValue 1.0) _returnvalue_yaw)) false false)
    (elif (`self.LeftClick`)
      (`self.K2_SetActorLocation` (+ (* (* (`SceneComponent.GetRightVector` (`self.Arrow`)) (* AxisValue -1.0)) (`self.MoveSpeed`)) (`self.K2_GetActorLocation`))))))

(event `Key|MouseScrollDown`
  (params (Key :type "Key Structure"))
  (bind _springarm (`self.SpringArm`))
  ;[1 1 1] MouseWheelControl
  (:`Pressed`
    (set `SpringArmComponent.TargetArmLength` (+ (`SpringArmComponent.TargetArmLength` _springarm) (`self.SpeedWheel`)) _springarm)))

(event `Key|MouseScrollUp`
  (params (Key :type "Key Structure"))
  (bind _springarm (`self.SpringArm`))
  ;[1 1 1] MouseWheelControl
  (:`Pressed`
    (set `SpringArmComponent.TargetArmLength` (- (`SpringArmComponent.TargetArmLength` _springarm) (`self.SpeedWheel`)) _springarm)))

(event `InputAxisKey|MouseY`
  (params (AxisValue :type "Float (single-precision)"))
  (bind _springarm (`self.SpringArm`))
  (bind (_returnvalue_roll _returnvalue_pitch _returnvalue_yaw) (`KismetMathLibrary.BreakRotator` (`SceneComponent.K2_GetComponentRotation` _springarm)))
  ;[1 1 1] Rotation
  (if (`self.RightClick`)
    (`SceneComponent.K2_SetWorldRotation` _springarm (`KismetMathLibrary.MakeRotator` 0.0 (+ (* AxisValue 1.0) _returnvalue_pitch) _returnvalue_yaw) false false)
    (elif (`self.LeftClick`)
      (`self.K2_SetActorLocation` (+ (* (* (`SceneComponent.GetForwardVector` (`self.Arrow`)) (* AxisValue -1.0)) (`self.MoveSpeed`)) (`self.K2_GetActorLocation`))))))

(event `Key|LeftMouseButton`
  (params (Key :type "Key Structure"))
  ;[1 1 1] Click?
  (:`Pressed`
    (set `self.LeftClick` true))
  (:`Released`
    (set `self.LeftClick` false)))

(event `Key|RightMouseButton`
  (params (Key :type "Key Structure"))
  ;[1 1 1] Click?
  (:`Pressed`
    (set `self.RightClick` true))
  (:`Released`
    (set `self.RightClick` false)))

(fn `UserConstructionScript`)